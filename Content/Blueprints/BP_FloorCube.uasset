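; BP_FloorCube is a clickable floor cube that can switch its mesh between grey and highlighted materials.
; Clicking the mesh casts the player pawn to BP_OrbitCameraPawn, then clears the highlight via SetHighlighted.
; The CanInteractWithCubes check has empty branches, so it does not gate that reset.
; SetHighlighted swaps the first material slot, but nothing in this Blueprint turns the highlight on.
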(event `self.StaticMesh.OnClicked`
  (params (TouchedComponent :type "PrimitiveComponent Object Reference") (ButtonPressed :type "Key Structure"))
  (bind _asbp_orbit_camera_pawn (cast `/Game/Blueprints/BP_OrbitCameraPawn` (`GameplayStatics.GetPlayerPawn` 0)))
  (if (`/Game/Blueprints/BP_OrbitCameraPawn.CanInteractWithCubes` _asbp_orbit_camera_pawn)
    _
    (else
      _))
  (`self.SetHighlighted` false))

(fn `SetHighlighted`
  (params (IsHighlighted :type Boolean))
  (if IsHighlighted
    (`PrimitiveComponent.SetMaterial` (`self.StaticMesh`) 0 "/Game/Materials/M_Highlight.M_Highlight")
    (else
      (`PrimitiveComponent.SetMaterial` (`self.StaticMesh`) 0 "/Game/Materials/M_Grey.M_Grey"))))

(fn `UserConstructionScript`)