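; Orbit camera pawn for inspecting and selecting tower floor cubes, paired with a WBP_FloorUI widget created on BeginPlay.
; Left-drag rotates the spring arm, right-drag pans it and the wheel zooms.
; A timed double-click traces under the cursor, highlights a cube in the UI's selected tower and fills the data panel.
; Tick eases the camera toward that cube, while a single click clears selection and eases back to the start focus.
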(event `self.ReceiveBeginPlay`
  (bind _returnvalue (`GameplayStatics.GetPlayerController` 0))
  (set `self.Default Focus Location` (`SceneComponent.K2_GetComponentLocation` (`self.SpringArm`)))
  (bind _returnvalue_2 (`|CreateWidget` "/Game/Blueprints/WBP_FloorUI.WBP_FloorUI_C"))
  (set `self.FloorUI_Ref` _returnvalue_2)
  (`UserWidget.AddToViewport` _returnvalue_2 0)
  (bind _output_get (set `PlayerController.bShowMouseCursor` true _returnvalue))
  (`WidgetBlueprintLibrary.SetInputMode_GameAndUIEx` _returnvalue null "DoNotLock" _output_get))

(event `Key|MouseScrollUp`
  (params (Key :type "Key Structure"))
  (bind _springarm (`self.SpringArm`))
  (:`Pressed`
    (set `self.IsFocusing` false)
    (set `self.Is Returning` false)
    (set `SpringArmComponent.TargetArmLength` (- (`SpringArmComponent.TargetArmLength` _springarm) 100.0) _springarm)))

(event `Key|MouseScrollDown`
  (params (Key :type "Key Structure"))
  (bind _springarm (`self.SpringArm`))
  (:`Pressed`
    (set `self.IsFocusing` false)
    (set `self.Is Returning` false)
    (set `SpringArmComponent.TargetArmLength` (+ (`SpringArmComponent.TargetArmLength` _springarm) 100.0) _springarm)))

(event `Key|LeftMouseButton`
  (params (Key :type "Key Structure"))
  (bind _returnvalue (`KismetSystemLibrary.GetGameTimeInSeconds`))
  (bind _selectedcube (`self.SelectedCube`))
  (bind _selectedcube_2 (`self.SelectedCube`))
  (bind _floorui_ref (`self.FloorUI_Ref`))
  (bind _floorui_ref_2 (`self.FloorUI_Ref`))
  (bind _floortext (`/Game/Blueprints/WBP_FloorUI.FloorText` _floorui_ref_2))
  (:`Pressed`
    (set `self.IsLeftMousePressed` true)
    (if (<= (- _returnvalue (`self.LastClickTime`)) 0.3)
      (bind _asbp_orbit_camera_pawn (cast `/Game/Blueprints/BP_OrbitCameraPawn` (`GameplayStatics.GetPlayerPawn` 0)))
      (if (`/Game/Blueprints/BP_OrbitCameraPawn.CanInteractWithCubes` _asbp_orbit_camera_pawn)
        (bind _asbp_floor_cube (cast `/Game/Blueprints/BP_FloorCube` (`.HitActor` (`GameplayStatics.BreakHitResult` (`PlayerController.GetHitResultUnderCursorByChannel` (`GameplayStatics.GetPlayerController` 0) "TraceTypeQuery1" true)))))
        (if (`KismetStringLibrary.EqualEqual_StrStr` (`/Game/Blueprints/BP_FloorCube.TowerID` _asbp_floor_cube) (`/Game/Blueprints/WBP_FloorUI.SelectedTower` _floorui_ref))
          (`/Engine/EditorBlueprintResources/StandardMacros.IsValid` _selectedcube
            (:`Is Valid`
              (`/Game/Blueprints/BP_FloorCube.SetHighlighted` _selectedcube false))
            (:`Is Not Valid`
              _))
          (bind _output_get (set `self.SelectedCube` _asbp_floor_cube))
          (`/Game/Blueprints/BP_FloorCube.SetHighlighted` _output_get true)
          (`/Game/Blueprints/WBP_FloorUI.UpdateDataPanel` _floorui_ref (`/Game/Blueprints/BP_FloorCube.Unit` _asbp_floor_cube) (`/Game/Blueprints/BP_FloorCube.TowerID` _asbp_floor_cube) (`/Game/Blueprints/BP_FloorCube.FloorNumber` _asbp_floor_cube) (`KismetMathLibrary.Conv_IntToDouble` (`/Game/Blueprints/BP_FloorCube.Size` _asbp_floor_cube)) (`/Game/Blueprints/BP_FloorCube.Value` _asbp_floor_cube))
          (set `self.TargetFocusLocation` (`self.K2_GetActorLocation` (`self.SelectedCube`)))
          (set `self.IsFocusing` true)
          (set `self.Is Returning` false)))
      (else
        (set `self.LastClickTime` _returnvalue)
        (set `self.IsFocusing` false)
        (set `self.Is Returning` true)
        (set `self.TargetFocusLocation` (`SceneComponent.K2_GetComponentLocation` (`self.SpringArm`)))
        (`/Engine/EditorBlueprintResources/StandardMacros.IsValid` _selectedcube_2
          (:`Is Valid`
            (`/Game/Blueprints/BP_FloorCube.SetHighlighted` _selectedcube_2 false)
            (`/Game/Blueprints/WBP_FloorUI.UpdateDataPanel` _floorui_ref_2 "" "" 0 0.0 0.0))
          (:`Is Not Valid`
            _))
        (if (`KismetStringLibrary.NotEqual_StrStr` (`/Game/Blueprints/WBP_FloorUI.SelectedTower` _floorui_ref_2))
          (`TextBlock.SetText` _floortext "Double Click Cube To Select")
          (set `self.SelectedCube` null)
          (else
            (`TextBlock.SetText` _floortext "Select a Tower To Start")
            (set `self.SelectedCube` null))))))
  (:`Released`
    (set `self.IsLeftMousePressed` false)))

(event `Key|RightMouseButton`
  (params (Key :type "Key Structure"))
  (:`Pressed`
    (set `self.IsRightMouseDown` true)
    (set `self.IsFocusing` false)
    (set `self.Is Returning` false))
  (:`Released`
    (set `self.IsRightMouseDown` false)))

(event `FocusToCube`
  (params (TargetCube :type "/Game/Blueprints/BP_FloorCube Object Reference"))
  (set `self.TargetFocusLocation` (`self.K2_GetActorLocation` TargetCube))
  (set `self.IsFocusing` true))

(event `self.ReceiveTick`
  (params (DeltaSeconds :type "Float (single-precision)"))
  (bind _returnvalue (`GameplayStatics.GetWorldDeltaSeconds`))
  (bind _returnvalue_2 (`GameplayStatics.GetWorldDeltaSeconds`))
  (bind _springarm (`self.SpringArm`))
  (bind _springarm_2 (`self.SpringArm`))
  (bind _targetfocuslocation (`self.TargetFocusLocation`))
  (bind _springarm_3 (`self.SpringArm`))
  (bind _default_focus_location (`self.Default Focus Location`))
  (bind _selectedcube (`self.SelectedCube`))
  (bind (_deltax _deltay) (`PlayerController.GetInputMouseDelta` (`GameplayStatics.GetPlayerController` 0)))
  (bind (_deltax_2 _deltay_2) (`PlayerController.GetInputMouseDelta` (`GameplayStatics.GetPlayerController` 0)))
  (bind _returnvalue_3 (`KismetMathLibrary.VInterpTo` (`SceneComponent.K2_GetComponentLocation` _springarm_3) _default_focus_location _returnvalue 6.0))
  (bind _returnvalue_4 (`KismetMathLibrary.VInterpTo` (`SceneComponent.K2_GetComponentLocation` _springarm) _targetfocuslocation _returnvalue_2 6.0))
  (`|ExecutionSequence`
    (:`then_0`
      (if (`self.IsLeftMousePressed`)
        (`SceneComponent.K2_AddRelativeRotation` (`self.SpringArm`) (`KismetMathLibrary.MakeRotator` 0.0 _deltay _deltax) false false)))
    (:`then_1`
      (if (`self.IsRightMouseDown`)
        (`SceneComponent.K2_AddLocalOffset` (`self.SpringArm`) (`KismetMathLibrary.MakeVector` 0.0 _deltax_2 _deltay_2) false false)))
    (:`then_2`
      (if (`self.IsFocusing`)
        (set `SpringArmComponent.TargetArmLength` (`KismetMathLibrary.FInterpTo` (`SpringArmComponent.TargetArmLength` _springarm) 500.0 _returnvalue_2 6.0) _springarm_2)
        (`SceneComponent.K2_SetWorldLocation` _springarm_2 _returnvalue_4 false false)
        (if (<= (`KismetMathLibrary.Vector_Distance` _returnvalue_4 _targetfocuslocation) 2.0)
          _)
        (elif (`self.Is Returning`)
          (set `SpringArmComponent.TargetArmLength` (`KismetMathLibrary.FInterpTo` (`SpringArmComponent.TargetArmLength` _springarm_3) 1000.0 _returnvalue 6.0) _springarm_3)
          (`SceneComponent.K2_SetWorldLocation` _springarm_3 _returnvalue_3 false false)
          (if (< (`KismetMathLibrary.Vector_Distance` _returnvalue_3 _default_focus_location) 2.0)
            (`/Engine/EditorBlueprintResources/StandardMacros.IsValid` _selectedcube
              (:`Is Valid`
                (`/Game/Blueprints/BP_FloorCube.SetHighlighted` _selectedcube false)
                (set `self.SelectedCube` null)
                (set `self.Is Returning` false)))))))))

(fn `UserConstructionScript`)